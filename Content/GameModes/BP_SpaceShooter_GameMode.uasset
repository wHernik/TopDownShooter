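; Space shooter game mode that spawns aliens continuously at random points in the level.
; Shortly after BeginPlay, NewWave increments the wave counter and starts a looping timer on SpawnWave, with nothing here stopping it or advancing further waves.
; Each tick of that timer calls SpawnSpider, which picks a random TargetPoint actor and spawns a BP_Alien at its transform if valid.
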(event Custom|SpawnWave
  (CallFunction|SpawnSpider))

(event EventBeginPlay
  (Utilities|FlowControl|Delay 2.0)
  (CallFunction|NewWave))

(fn ConstructionScript)

(fn NewWave
  (Math|Integer|IncrementInt (Variables|Default|GetCurrentWave)
    (:%20%20
      (Utilities|Time|SetTimerbyFunctionName 0 "SpawnWave" 1.0 true))))

(fn RandomSpawnPoint
  (bind _outactors (Actor|GetAllActorsOfClass "/Script/Engine.TargetPoint"))
  (return (Utilities|Array|Get(acopy) _outactors (Math|Random|RandomIntegerinRange 0 (Utilities|Array|LastIndex _outactors)))))

(fn SpawnSpider
  (bind _spawnpoint (CallFunction|RandomSpawnPoint))
  (Utilities|IsValid _spawnpoint
    (:Is%20Valid
      (Game|SpawnActorfromClass "/Game/Blueprints/AI/BP_Alien.BP_Alien_C" (Transformation|GetActorTransform _spawnpoint) "Undefined" 0 0))))