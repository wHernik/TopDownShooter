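; Wave counter Blueprint for a space shooter that tracks the current wave number.
; BeginPlay calls NewWave to increment CurrentWave, then runs a two-second Delay with nothing after it.
; UpdateCurrentWave checks that the game mode is BP_SpaceShooter_GameMode and returns the number as text prefixed with "Wave".
; No enemy spawning or further wave progression is implemented here.
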(event EventBeginPlay
  (CallFunction|NewWave)
  (Utilities|FlowControl|Delay 2.0))

(fn ConstructionScript)

(fn NewWave
  (Variables|Default|SetCurrentWave (+ (Variables|Default|GetCurrentWave) 1))
  (return))

(fn UpdateCurrentWave
  (Utilities|Casting|CastToBP_SpaceShooter_GameMode (Game|GetGameMode))
  (return (Utilities|Text|ToText(String) (Utilities|String|Append "Wave" (Utilities|String|ToString(Integer) (Variables|Default|GetCurrentWave))))))